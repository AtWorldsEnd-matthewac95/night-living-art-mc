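; Artwork puzzle actor that accepts pieces into mapped positions and can yield an inventory item.
; On BeginPlay it increments the Counter's total artwork count, retrying once if that fails.
; OccupyPositionAndGetInventoryItem checks the piece's mapping to this actor, occupies and verifies the position, then looks for a SwissBlockPositionMesh with position NONE.
; It returns that mesh's first child as the ItemBase item, alongside placement and correctness results.
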(event `self.ReceiveBeginPlay`
  (bind _counter (`self.Counter`))
  (bind _returnvalue (`ArtworkCounter.IncrementTotalArtworkCount` _counter))
  (if (not _returnvalue)
    (`ArtworkCounter.IncrementTotalArtworkCount` _counter)))

(fn `OccupyPositionAndGetInventoryItem`
  (params (piece :type "SwissBlockPiece Object Reference") (useLocation :type Boolean) (worldLocation :type "Vector Structure"))
  (returns (occupySuccess :type Boolean) (itemSuccess :type Boolean) (inventoryItem :type "/Game/InventorySystem/ItemBase_Component Object Reference") (isCorrect :type Boolean) (occupiedPosition :type Byte))
  (if (`.ReturnValue` (`SwissBlockPiece.FindMappedPosition` piece self))
    (bind (_iscorrect _occupiedposition _returnvalue) (`self.OccupyPositionAndVerifyCorrect` piece useLocation worldLocation))
    (if _returnvalue
      (for _array_element (`self.K2_GetComponentsByClass` "/Script/DepoReco.SwissBlockPositionMesh")
        (if (`|EnumEquality` "SBP_NONE" (`SwissBlockPositionMesh.GetSBPosition` _array_element))
          (bind _asitem_base_component (cast `/Game/InventorySystem/ItemBase_Component` (`SceneComponent.GetChildComponent` _array_element 0))
            (:`then`
              (return true true _asitem_base_component _iscorrect _occupiedposition))
            (:`CastFailed`
              (return true false null _iscorrect _occupiedposition)))))
      (return true false null _iscorrect _occupiedposition)
      (else
        (return false false null _iscorrect _occupiedposition)))
    (else
      (return false false null false 0))))

(fn `UserConstructionScript`)