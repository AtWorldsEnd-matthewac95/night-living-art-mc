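; Player controller for an artwork game that manages the HUD, level audio and the win or lose ending.
; BeginPlay creates the inventory HUD, hiding it on the main menu, and plays title or level music.
; Releasing Interact refreshes correct and total counts from ArtworkCounter.
; Pressing Exit while the externally supplied overlap flag is true fades the HUD, shows WinScreen if all artworks are correct, otherwise LoseScreen, then pauses with UI-only input.
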(event `self.ReceiveBeginPlay`
  (bind _returnvalue (`|CreateWidget` "/Game/InventorySystem/InventoryUI/InventoryHUD.InventoryHUD_C"))
  (bind _output_get (set `self.HUDRef` _returnvalue))
  (`UserWidget.AddToViewport` _output_get 0)
  (bind _returnvalue_2 (`GameplayStatics.GetCurrentLevelName` true))
  (if (`KismetStringLibrary.EqualEqual_StrStr` _returnvalue_2 "MainMenuLevel")
    (`Widget.SetVisibility` (`self.HUDRef`) "Hidden")
    (`GameplayStatics.PlaySound2D` (`self.TitleScreenSound`) 0.1 1.0 0.0 null null)
    (else
      (`Widget.SetVisibility` (`self.HUDRef`) "Visible")
      (`GameplayStatics.PlaySound2D` (`self.LevelSound`) 0.5 1.0 0.0 null null))))

(event `InputAction|Interact` :consume false
  (params (Key :type "Key Structure"))
  (bind _artworkcounter (`self.ArtworkCounter`))
  (bind _hudref (`self.HUDRef`))
  (:`Released`
    (set `/Game/InventorySystem/InventoryUI/InventoryHUD.Denominator` (`KismetStringLibrary.Conv_IntToString` (`ArtworkCounter.GetTotalArtworkCount` _artworkcounter)) _hudref)
    (set `/Game/InventorySystem/InventoryUI/InventoryHUD.Numerator` (`KismetStringLibrary.Conv_IntToString` (`ArtworkCounter.GetCorrectArtworkCount` _artworkcounter)) _hudref)
    (`/Game/InventorySystem/InventoryUI/InventoryHUD.UpdatePaintingCounts` _hudref)))

(event `InputAction|Exit`
  (params (Key :type "Key Structure"))
  (bind _returnvalue (`GameplayStatics.GetPlayerController` 0))
  (bind _hudref (`self.HUDRef`))
  (bind _artworkcounter (`self.ArtworkCounter`))
  (bind _fade (`/Game/InventorySystem/InventoryUI/InventoryHUD.Fade` _hudref))
  (:`Pressed`
    (if (`self.IsOverlapping`)
      (`UserWidget.PlayAnimation` _hudref _fade 0.0 1 "Forward" 1.0 false)
      (`KismetSystemLibrary.Delay` (`WidgetAnimation.GetEndTime` _fade))
      (if (== (`ArtworkCounter.GetCorrectArtworkCount` _artworkcounter) (`ArtworkCounter.GetTotalArtworkCount` _artworkcounter))
        (bind _returnvalue_2 (`|CreateWidget` "/Game/InventorySystem/InventoryUI/WinScreen.WinScreen_C"))
        (bind _output_get (set `self.WinScreenRef` _returnvalue_2))
        (`UserWidget.AddToViewport` _output_get 0)
        (`WidgetBlueprintLibrary.SetInputMode_UIOnlyEx` _returnvalue (`self.WinScreenRef`))
        (else
          (bind _returnvalue_3 (`|CreateWidget` "/Game/InventorySystem/InventoryUI/LoseScreen.LoseScreen_C"))
          (bind _output_get_2 (set `self.LoseScreenRef` _returnvalue_3))
          (`UserWidget.AddToViewport` _output_get_2 0)
          (`WidgetBlueprintLibrary.SetInputMode_UIOnlyEx` _returnvalue (`self.LoseScreenRef`))))
      (set `PlayerController.bShowMouseCursor` true _returnvalue)
      (`GameplayStatics.SetGamePaused` true))))

(fn `Get Is Overlapping`
  (params (IsOverlapping :type Boolean))
  (set `self.IsOverlapping` IsOverlapping)
  (return))

(fn `UserConstructionScript`)