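; AI "crazy man" character that wanders the navmesh, flees the player and periodically plays random crazy sounds.
; Tick starts a new move when idle: away from the player if inside RunAwayRadius, otherwise to a random reachable point.
; A looping timer keeps the Character component's yaw turned toward the player, even while moving.
; The component's material at BeginPlay identifies the guitar man variant, which has its own sound pool and longer delay.
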(event `self.ReceiveBeginPlay`
  (bind _asbp_first_person_character (cast `/Game/Blueprints/BP_FirstPersonCharacter` (`GameplayStatics.GetPlayerCharacter` 0)))
  (set `self.BP First Person Character` _asbp_first_person_character)
  (`KismetSystemLibrary.K2_SetTimer` null "FacePlayer" 0.01 true)
  ;[1 1 1] Checks Which Man This AI Is
  (if (== (`PrimitiveComponent.GetMaterial` (`self.Character`) 0) (`self.GuitarManMaterial`))
    (set `self.IsGuitarMan` true)
    (else
      (set `self.IsGuitarMan` false))))

(event `RunAway`
  (bind _returnvalue (`self.K2_GetActorLocation`))
  ;[0.04338 0.4948 0] RunAway
  (`|AIMoveTo` self (`NavigationSystemV1.K2_GetRandomLocationInNavigableRadius` (`KismetMathLibrary.MakeVector` (.x (+ _returnvalue (* (`KismetMathLibrary.GetForwardVector` (`KismetMathLibrary.FindLookAtRotation` _returnvalue (`self.K2_GetActorLocation` (`self.BP First Person Character`)))) -1000.0))) (.y (+ _returnvalue (* (`KismetMathLibrary.GetForwardVector` (`KismetMathLibrary.FindLookAtRotation` _returnvalue (`self.K2_GetActorLocation` (`self.BP First Person Character`)))) -1000.0))) (.z _returnvalue)) 2000.0 null null) null 5.0 true
    (:`OnSuccess`
      _)
    (:`OnFail`
      _))
  (set `self.IsMoving` false))

(event `self.ReceiveTick`
  (params (DeltaSeconds :type "Float (single-precision)"))
  (bind _returnvalue (`KismetMathLibrary.RandomFloatInRange` 5.0 10.0))
  ;[0.04338 0.4948 0] MoveTo
  (`|ExecutionSequence`
    (:`then_0`
      (if (not (`self.IsMoving`))
        (`KismetSystemLibrary.Delay` 0.001)
        (set `self.IsMoving` true)
        (if (`PrimitiveComponent.IsOverlappingActor` (`self.RunAwayRadius`) (`self.BP First Person Character`))
          (`Controller.StopMovement` (`AIBlueprintHelperLibrary.GetAIController` self))
          (`self.RunAway`)
          (else
            (`|AIMoveTo` self (`NavigationSystemV1.K2_GetRandomReachablePointInRadius` (`self.K2_GetActorLocation`) 2000.0 null null) null 5.0 true
              (:`OnSuccess`
                _)
              (:`OnFail`
                _))
            (set `self.IsMoving` false)))))
    (:`then_1`
      ;[0.04338 0.4948 0] Play The Crazy Sound After A Delay Between 5 And 10 Seconds
      (if (`self.IsGuitarMan`)
        (`KismetSystemLibrary.Delay` (+ _returnvalue 2.0))
        (else
          (`KismetSystemLibrary.Delay` _returnvalue)))
      (`self.PlayCrazySound`))))

(event `FacePlayer`
  (bind _character (`self.Character`))
  (bind (_returnvalue_roll _returnvalue_pitch) (`KismetMathLibrary.BreakRotator` (`SceneComponent.K2_GetComponentRotation` _character)))
  (bind (_returnvalue_roll_2 _returnvalue_pitch_2 _returnvalue_yaw) (`KismetMathLibrary.BreakRotator` (`KismetMathLibrary.FindLookAtRotation` (`SceneComponent.K2_GetComponentLocation` _character) (`self.K2_GetActorLocation` (`self.BP First Person Character`)))))
  (bind (_returnvalue_roll_3 _returnvalue_pitch_3 _returnvalue_yaw_2) (`KismetMathLibrary.BreakRotator` (`KismetMathLibrary.RInterpTo` (`SceneComponent.K2_GetComponentRotation` _character) (`KismetMathLibrary.MakeRotator` _returnvalue_roll_2 _returnvalue_pitch_2 (+ _returnvalue_yaw -90.0)) (`GameplayStatics.GetWorldDeltaSeconds`) 1000000.0)))
  ;[0.04338 0.4948 0] FacePlayer
  (`SceneComponent.K2_SetWorldRotation` (`self.Character`) (`KismetMathLibrary.MakeRotator` _returnvalue_roll _returnvalue_pitch _returnvalue_yaw_2) false false))

(event `PlayCrazySound`
  ;[0.04338 0.4948 0] Set & Play Crazy Man Audio
  (if (`self.IsGuitarMan`)
    (switch `int` (`KismetMathLibrary.RandomIntegerInRange` 0 5)
      (:`0`
        (`AudioComponent.SetSound` (`self.CrazyManAudioComponent`) "/Game/Audio/Crazy_10.Crazy_10"))
      (:`1`
        (`AudioComponent.SetSound` (`self.CrazyManAudioComponent`) "/Game/Audio/Crazy_11.Crazy_11"))
      (:`2`
        (`AudioComponent.SetSound` (`self.CrazyManAudioComponent`) "/Game/Audio/Crazy_12.Crazy_12"))
      (:`3`
        (`AudioComponent.SetSound` (`self.CrazyManAudioComponent`) "/Game/Audio/Crazy_13.Crazy_13"))
      (:`4`
        (`AudioComponent.SetSound` (`self.CrazyManAudioComponent`) "/Game/Audio/Crazy_14.Crazy_14"))
      (:`5`
        (`AudioComponent.SetSound` (`self.CrazyManAudioComponent`) "/Game/Audio/CRAZY_18.CRAZY_18")))
    (else
      (switch `int` (`KismetMathLibrary.RandomIntegerInRange` 0 8)
        (:`0`
          (`AudioComponent.SetSound` (`self.CrazyManAudioComponent`) "/Game/Audio/Crazy_1.Crazy_1"))
        (:`1`
          (`AudioComponent.SetSound` (`self.CrazyManAudioComponent`) "/Game/Audio/Crazy_2.Crazy_2"))
        (:`2`
          (`AudioComponent.SetSound` (`self.CrazyManAudioComponent`) "/Game/Audio/Crazy_3.Crazy_3"))
        (:`3`
          (`AudioComponent.SetSound` (`self.CrazyManAudioComponent`) "/Game/Audio/Crazy_4.Crazy_4"))
        (:`4`
          (`AudioComponent.SetSound` (`self.CrazyManAudioComponent`) "/Game/Audio/Crazy_5.Crazy_5"))
        (:`5`
          (`AudioComponent.SetSound` (`self.CrazyManAudioComponent`) "/Game/Audio/Crazy_6.Crazy_6"))
        (:`6`
          (`AudioComponent.SetSound` (`self.CrazyManAudioComponent`) "/Game/Audio/Crazy_7.Crazy_7"))
        (:`7`
          (`AudioComponent.SetSound` (`self.CrazyManAudioComponent`) "/Game/Audio/Crazy_8.Crazy_8"))
        (:`8`
          (`AudioComponent.SetSound` (`self.CrazyManAudioComponent`) "/Game/Audio/Crazy_9.Crazy_9")))))
  (`AudioComponent.Play` (`self.CrazyManAudioComponent`) 0.0))

(fn `UserConstructionScript`)